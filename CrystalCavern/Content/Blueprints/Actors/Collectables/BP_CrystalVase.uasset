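; Collectable crystal vase that spins in place with a yellow point light and flies to the player on pickup.
; A player overlap on the collision component stores the start transform values and plays a timeline.
; The timeline lerps the actor toward player pawn 0's current location each update while setting the vase mesh's world scale from its Scale track, ignoring the stored StartScale.
; The actor destroys itself when the timeline finishes.
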(event `self.ReceiveTick`
  (params (DeltaSeconds :type "Float (single-precision)"))
  (`SceneComponent.K2_AddLocalRotation` (`self.Vase`) (`KismetMathLibrary.MakeRotator` 0.0 0.0 (* (`self.RotationSpeed`) DeltaSeconds)) false false))

(event `self.Collision Component.OnComponentBeginOverlap`
  (params (OverlappedComponent :type "PrimitiveComponent Object Reference") (OtherActor :type "Actor Object Reference") (OtherComp :type "PrimitiveComponent Object Reference") (OtherBodyIndex :type Integer) (bFromSweep :type Boolean) (SweepResult :type "HitResult Structure (by ref)"))
  (`/Game/Blueprints/Libraries/CC_MacroLibrary.IsPlayer` OtherActor
    (:`isPlayer`
      (`self.StoreStartingValues`)
      (bind (_direction _alpha _scale) (`Timeline|Alpha Blend Timeline`)
        (:`Update`
          (`self.MoveToPlayer` _alpha)
          (`self.ScaleVase` _scale))
        (:`Finished`
          (`self.K2_DestroyActor`))))))

(fn `MoveToPlayer`
  (params (Alpha :type "Float (double-precision)"))
  (`self.K2_SetActorLocation` (`KismetMathLibrary.VLerp` (`self.Lerp Start Location`) (`self.K2_GetActorLocation` (`GameplayStatics.GetPlayerPawn` 0)) Alpha)))

(fn `ScaleVase`
  (params (Scale :type "Vector Structure"))
  (`SceneComponent.SetWorldScale3D` (`self.Vase`) Scale))

(fn `StoreStartingValues`
  (set `self.Lerp Start Location` (`self.K2_GetActorLocation`))
  (set `self.Start  Scale` (`self.GetActorScale3D`)))

(fn `UserConstructionScript`
  (`LightComponent.SetLightColor` (`self.PointLight`) (struct :`R` 1.0 :`G` 1.0 :`A` 1.0) true))