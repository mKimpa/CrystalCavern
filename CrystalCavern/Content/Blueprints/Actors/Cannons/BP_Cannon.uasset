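; BP_Cannon is a cannon actor that automatically fires BP_Projectile on a randomized interval.
; After a random delay between the minimal and maximum fire rate, it spawns a scaled projectile at the barrel's Projectile socket.
; A BarrelMove timeline then slides the barrel along its local Y axis, and its Cannon Fired event restarts the loop with a new delay.
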(event `self.ReceiveBeginPlay`
  (`KismetSystemLibrary.Delay` (`KismetMathLibrary.RandomFloatInRange` (`self.MinimalFireRate`) (`self.MaximumFireRate`)) :!label _label)
  (`self.Spawn Projectile`)
  (bind (_direction _cannon_barrel_location) (`Timeline|Barrel Move` :!via `PlayFromStart`)
    (:`Update`
      (`self.Move Cannon Barrel` _cannon_barrel_location))
    (:`Cannon Fired`
      (goto _label))))

(event `self.ReceiveTick`
  (params (DeltaSeconds :type "Float (single-precision)")))

(fn `Move Cannon Barrel`
  (params (`Cannon Barrrel Y Location` :type "Float (double-precision)"))
  (`SceneComponent.K2_SetRelativeLocation` (`self.CannonBarrel`) (`KismetMathLibrary.MakeVector` 0.0 `Cannon Barrrel Y Location`) false false))

(fn `Spawn Projectile`
  (`|SpawnActorFromClass` "/Game/Blueprints/Actors/Projectiles/BP_Projectile.BP_Projectile_C" (`KismetMathLibrary.MakeTransform` (.location (`SceneComponent.GetSocketTransform` (`self.CannonBarrel`) "Projectile" "RTS_World")) (.rotation (`SceneComponent.GetSocketTransform` (`self.CannonBarrel`) "Projectile" "RTS_World")) (`KismetMathLibrary.Conv_DoubleToVector` (`self.ProjectileScale`))) "Undefined" "OverrideRootScale" null null))

(fn `UserConstructionScript`)