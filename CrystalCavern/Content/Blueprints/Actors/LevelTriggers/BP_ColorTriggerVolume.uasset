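; BP_ColorTriggerVolume is a color-keyed level trigger that assigns a color to the player and breaks a bridge on a mismatch.
; On player overlap, a pawn with the unset key (transparent white) takes the volume's Color.
; A differing key applies damage with impulse to the mesh of the owning BP_Bridge and prints a debug string.
; The construction script tints the SpotLight to match Color.
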(event `self.ReceiveActorBeginOverlap`
  (params (OtherActor :type "Actor Object Reference"))
  (`/Game/Blueprints/Libraries/CC_MacroLibrary.IsPlayer` OtherActor
    (:`isPlayer`
      (bind _asbp_player_pawn (cast `/Game/Blueprints/Pawns/BP_PlayerPawn` OtherActor))
      (bind _colorkey (`/Game/Blueprints/Pawns/BP_PlayerPawn.GetColorKey` _asbp_player_pawn))
      (if (== _colorkey (struct :`R` 1.0 :`G` 1.0 :`B` 1.0))
        (`/Game/Blueprints/Pawns/BP_PlayerPawn.SetColorKey` _asbp_player_pawn (`self.Color`))
        (else
          (bind _colorkey_2 (`/Game/Blueprints/Pawns/BP_PlayerPawn.GetColorKey` _asbp_player_pawn))
          (if (!= _colorkey_2 (`self.Color`))
            (bind _asbp_bridge (cast `/Game/Blueprints/Actors/Bridges/BP_Bridge` (`self.GetOwner`)))
            (`DestructibleComponent.ApplyDamage` (`/Game/Blueprints/Actors/Bridges/BP_Bridge.Mesh` _asbp_bridge) 1.0 (0.0 0.0 0.0) (0.0 0.0 0.0) 1.0)
            (`KismetSystemLibrary.PrintString` "Hello")))))))

(fn `UserConstructionScript`
  (`LightComponent.SetLightColor` (`self.SpotLight`) (`self.Color`) true))