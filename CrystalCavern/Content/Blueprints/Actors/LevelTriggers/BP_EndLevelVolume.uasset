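; BP_EndLevelVolume is a level trigger that ends the current level when the player overlaps it.
; On overlap it adds the player controller's score to the total kept in BP_CC_GameInstance, then runs a camera fade.
; When the fade completes, it finds the current level in a LevelNames array and opens the next one by name, or prints "Game Over!" and quits on the last.
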(event `self.ReceiveActorBeginOverlap`
  (params (OtherActor :type "Actor Object Reference"))
  (`/Game/Blueprints/Libraries/CC_MacroLibrary.IsPlayer` OtherActor
    (:`isPlayer`
      (`self.SetTotalScore`)
      (`/Game/Blueprints/Libraries/CC_MacroLibrary.CameraFade`
        (:`Complete`
          (`self.LevelComplete`))))))

(fn `GetCurrentLevelIndex`
  (returns (`Current Level Index` :type Integer))
  (bind _returnvalue (`GameplayStatics.GetCurrentLevelName` true))
  (return (`KismetArrayLibrary.Array_Find` (`self.LevelNames`) _returnvalue)))

(fn `IsFinalLevel`
  (returns (`Is Final Level` :type Boolean))
  (return (== (`self.GetCurrentLevelIndex`) (`KismetArrayLibrary.Array_LastIndex` (`self.LevelNames`)))))

(fn `LevelComplete`
  (if (`self.IsFinalLevel`)
    (`KismetSystemLibrary.PrintString` "Game Over!")
    (`KismetSystemLibrary.QuitGame` null "Quit")
    (else
      (`self.LoadNextLevel`))))

(fn `LoadNextLevel`
  (`GameplayStatics.OpenLevel` (`KismetStringLibrary.Conv_StringToName` (`|GetArrayItem` (`self.LevelNames`) (+ (`self.GetCurrentLevelIndex`) 1)))))

(fn `SetTotalScore`
  (bind _asbp_player_controller (cast `/Game/Blueprints/PlayerController/BP_PlayerController` (`GameplayStatics.GetPlayerController` 0)))
  (bind _asbp_cc_game_instance (cast `/Game/Blueprints/BP_CC_GameInstance` (`GameplayStatics.GetGameInstance`)))
  (`/Game/Blueprints/BP_CC_GameInstance.SetTotalScore` _asbp_cc_game_instance (+ (`/Game/Blueprints/BP_CC_GameInstance.GetTotalScore` _asbp_cc_game_instance) (`/Game/Blueprints/PlayerController/BP_PlayerController.Score` _asbp_player_controller))))

(fn `UserConstructionScript`)