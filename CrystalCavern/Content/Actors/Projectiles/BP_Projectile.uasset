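; Projectile actor that kills the player pawn on hit and triggers a restart of the current level.
; On collision, CheckHitActor sorts the hit actor by exact class into Player, Vase or Other.
; Player hits notify the pawn, destroy the projectile, then call LevelRestart, which fades the camera and reopens the level after a Delay.
; Other hits just destroy the projectile, while the crystal vase branch has no handler.
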(event `self.CollisionComponent.OnComponentHit`
  (params (HitComponent :type "PrimitiveComponent Object Reference") (OtherActor :type "Actor Object Reference") (OtherComp :type "PrimitiveComponent Object Reference") (NormalImpulse :type "Vector Structure") (Hit :type "HitResult Structure (by ref)"))
  (`self.CheckHitActor` OtherActor
    (:`Player`
      (bind _asbp_player_pawn (cast `/Game/Pawns/BP_PlayerPawn` OtherActor))
      (`/Game/Pawns/BP_PlayerPawn.PlayerWasKilled` _asbp_player_pawn Hit)
      (`self.K2_DestroyActor`)
      (`self.Level Restart`))
    (:`Other`
      (`self.K2_DestroyActor`))))

(event `Level Restart`
  (bind _returnvalue (`GameplayStatics.GetCurrentLevelName` true))
  (`PlayerCameraManager.StartCameraFade` :`self` (`GameplayStatics.GetPlayerCameraManager` 0) :`ToAlpha` 1.0 :`Duration` 3.0 :`bHoldWhenFinished` true)
  (`KismetSystemLibrary.Delay` 3.0)
  (`GameplayStatics.OpenLevel` (`KismetStringLibrary.Conv_StringToName` _returnvalue)))

(fn `UserConstructionScript`)