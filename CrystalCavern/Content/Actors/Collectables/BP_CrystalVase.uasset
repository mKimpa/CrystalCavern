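; BP_CrystalVase is a collectable vase that spins in place under a yellow point light and flies into the player when touched.
; Tick yaws the mesh at RotationSpeed, while the construction script sets the light color.
; Overlap with a BP_PlayerPawn plays AlphaBlendTimeline, which lerps the actor from its current location toward player pawn 0's live position each update.
; The actor destroys itself when the timeline finishes, with no score or inventory change here.
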(event `self.ReceiveTick`
  (params (DeltaSeconds :type "Float (single-precision)"))
  (`SceneComponent.K2_AddLocalRotation` (`self.Vase`) (`KismetMathLibrary.MakeRotator` 0.0 0.0 (* (`self.RotationSpeed`) DeltaSeconds)) false false))

(event `self.Collision Component.OnComponentBeginOverlap`
  (params (OverlappedComponent :type "PrimitiveComponent Object Reference") (OtherActor :type "Actor Object Reference") (OtherComp :type "PrimitiveComponent Object Reference") (OtherBodyIndex :type Integer) (bFromSweep :type Boolean) (SweepResult :type "HitResult Structure (by ref)"))
  (if (== (`GameplayStatics.GetObjectClass` OtherActor) "/Game/Pawns/BP_PlayerPawn.BP_PlayerPawn_C")
    (bind (_direction _alpha) (`Timeline|Alpha Blend Timeline`)
      (:`Update`
        (`self.Move To Player` _alpha))
      (:`Finished`
        (`self.K2_DestroyActor`)))))

(fn `Move To Player`
  (params (Alpha :type "Float (double-precision)"))
  (`self.K2_SetActorLocation` (`KismetMathLibrary.VLerp` (`self.K2_GetActorLocation`) (`self.K2_GetActorLocation` (`GameplayStatics.GetPlayerPawn` 0)) Alpha)))

(fn `UserConstructionScript`
  (`LightComponent.SetLightColor` (`self.PointLight`) (struct :`R` 1.0 :`G` 1.0 :`A` 1.0) true))